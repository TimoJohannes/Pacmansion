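; Coin pickup actor for a Pac-Man style game that respawns after being collected.
; On capsule overlap with the Pacman character, it adds an audio component, calls TouchCoin on the character, hides its sphere and destroys its capsule.
; After a delay it spawns a fresh Coin at the saved transform and destroys itself.
; A coin-counting chain exists but is unconnected.
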(event OnComponentBeginOverlap(Capsule)
  (params (OtherActor :type Actor%20Object%20Reference) (OtherComp :type Primitive%20Component%20Object%20Reference) (OtherBodyIndex :type Integer) (bFromSweep :type Boolean) (SweepResult :type Hit%20Result%20Structure%20%28by%20ref%29))
  ;[1 1 1] Touch Character - Coin disappears and respawns after time
  (bind _aspacman (Utilities|Casting|CastToPacman OtherActor))
  (AddComponent|AddAudioComponent false)
  (Default|TouchCoin _aspacman) ; Calls Touch Coin Method on First Person Character
  (Variables|Default|SetCoinLocation (Transformation|GetActorTransform))
  (Rendering|SetVisibility (Variables|Default|GetSphere) false false)
  (Components|DestroyComponent (Variables|Default|GetCapsule)) ; Disables Collision (not workin?)
  (Utilities|FlowControl|Delay 1e+01) ; Respawn Time of Coin
  (Game|SpawnActorfromClass "Coin_C" (Variables|Default|GetCoinLocation) "AlwaysSpawn" 0 0) ; Spawns new Coin at old Location
  (Actor|DestroyActor) ; Destroys old Coin
)

(fn ConstructionScript)